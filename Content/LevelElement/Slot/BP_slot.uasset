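; BP_slot is a clickable empty slot in the level where the player opens a tower selection menu.
; On BeginPlay it passes itself as EmptySlot to the WB_ChooseTower inside its widget component.
; Cursor events on the Slot component swap hover, idle and clicked materials; a click also sets GameMode_personal's MoveScreen to false and toggles the widget's visibility.
; An older viewport-widget approach remains as unconnected code.
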(event `self.ReceiveBeginPlay`
  (bind _aswb_choose_tower (cast `/Game/HUV/WB_ChooseTower` (`WidgetComponent.GetUserWidgetObject` (`self.Widget`))))
  (set `/Game/HUV/WB_ChooseTower.EmptySlot` self _aswb_choose_tower))

(event `self.Slot.OnBeginCursorOver`
  (params (TouchedComponent :type "PrimitiveComponent Object Reference"))
  (`PrimitiveComponent.SetMaterial` (`self.Slot`) 0 "/Game/LevelElement/Slot/MaterialSlot/M_SlotMouseOver.M_SlotMouseOver"))

(event `self.Slot.OnEndCursorOver`
  (params (TouchedComponent :type "PrimitiveComponent Object Reference"))
  (`PrimitiveComponent.SetMaterial` (`self.Slot`) 0 "/Game/LevelElement/Slot/MaterialSlot/M_SlotMouseOut.M_SlotMouseOut"))

(event `self.Slot.OnClicked`
  (params (TouchedComponent :type "PrimitiveComponent Object Reference") (ButtonPressed :type "Key Structure"))
  (bind _widget (`self.Widget`))
  (bind _asgame_mode_personal (cast `/Game/TD_blueprint/GameMode_personal` (`GameplayStatics.GetGameMode`)))
  (set `/Game/TD_blueprint/GameMode_personal.MoveScreen` false _asgame_mode_personal)
  (`PrimitiveComponent.SetMaterial` (`self.Slot`) 0 "/Game/LevelElement/Slot/MaterialSlot/M_SlotMouseCliked.M_SlotMouseCliked")
  (if (`SceneComponent.IsVisible` (`self.Widget`))
    (`SceneComponent.SetVisibility` _widget false false)
    (else
      (`SceneComponent.SetVisibility` _widget true false))))

(event `self.Slot.OnReleased`
  (params (TouchedComponent :type "PrimitiveComponent Object Reference") (ButtonReleased :type "Key Structure"))
  (`PrimitiveComponent.SetMaterial` (`self.Slot`) 0 "/Game/LevelElement/Slot/MaterialSlot/M_SlotMouseOver.M_SlotMouseOver"))

(fn `UserConstructionScript`)