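; Projectile Blueprint that temporarily slows enemies it overlaps.
; On overlap it runs the parent's overlap logic, then casts the other actor to BP_EnnemyParent.
; It saves that enemy's MaxWalkSpeed, divides it by a fixed factor, and restores the saved value after a Delay on the projectile itself.
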(event `self.ReceiveActorBeginOverlap`
  (params (OtherActor :type "Actor Object Reference"))
  (`|ExecutionSequence`
    (:`then_0`
      (`parent.ReceiveActorBeginOverlap` OtherActor))
    (:`then_1`
      (bind _asbp_ennemy_parent (cast `/Game/Enemies/BP_EnnemyParent` OtherActor))
      (bind _charactermovement (`Character.CharacterMovement` _asbp_ennemy_parent))
      (bind _output_get (set `self.Initial Max Walk Speed` (`CharacterMovementComponent.MaxWalkSpeed` _charactermovement)))
      (set `CharacterMovementComponent.MaxWalkSpeed` (/ _output_get 1.2) _charactermovement)
      (`KismetSystemLibrary.Delay` 4.0)
      (set `CharacterMovementComponent.MaxWalkSpeed` (`self.Initial Max Walk Speed`) _charactermovement))))

(fn `UserConstructionScript`
  (`parent.UserConstructionScript`))